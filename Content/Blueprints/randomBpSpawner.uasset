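; A construction-script spawner that scatters a set number of copies of a chosen Blueprint class across the ground within a box around the actor.
; Each random point gets a vertical line trace against WorldStatic objects, and only hits produce a child actor component.
; Each child sits at the hit height plus a random vertical offset, takes a random yaw, and then receives the class.
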(event EventBeginPlay)

(event Collision|EventActorBeginOverlap
  (params (OtherActor :type Actor%20Object%20Reference)))

(event EventTick
  (params (DeltaSeconds :type Float%20%28single-precision%29)))

(fn ConstructionScript
  (bind _defaultsceneroot (Variables|Default|GetDefaultSceneRoot))
  (bind _returnvalue (Transformation|GetWorldLocation _defaultsceneroot))
  (for _index (range 1 (Variables|Default|Getnumber))
    (CallFunction|AddBP (+ (Math|Random|RandomPointinBoundingBox (Math|Vector|MakeVector 0.0 0.0 0.0) (Math|Vector|MakeVector (Variables|Default|GetxSize) (Variables|Default|GetySize) (Variables|Default|GetzSize))) _returnvalue) _returnvalue (Variables|Default|GetbpClass))))

(fn AddBP
  (params (position :type Vector) (worldPosition :type Vector) (bpClass :type Actor%20Class%20Reference))
  (bind (_x _y) (Math|Vector|BreakVector position))
  (Variables|Default|SetlocalbpClass bpClass)
  (LocalVariables|Setwp worldPosition)
  (bind (_outhit _returnvalue) (Collision|LineTraceForObjects (Math|Vector|MakeVector _x _y 2e+04) (Math|Vector|MakeVector _x _y -5e+03) (Utilities|Array|MakeArray "ObjectTypeQuery1") false 0 "None"))
  (if _returnvalue
    (bind _returnvalue_2 (AddComponent|AddChildActorComponent false (Math|Conversions|ToTransform(Vector) (- (Math|Vector|MakeVector (.X (Math|Vector|BreakVector (.Location (Collision|BreakHitResult _outhit)))) (.Y (Math|Vector|BreakVector (.Location (Collision|BreakHitResult _outhit)))) (+ (.Z (Math|Vector|BreakVector (.Location (Collision|BreakHitResult _outhit)))) (Math|Random|RandomFloatinRange (Variables|Default|GetzFloor) (Variables|Default|GetzCeil)))) (LocalVariables|Getwp)))))
    (Transformation|SetWorldRotation _returnvalue_2 (Math|Rotator|MakeRotator 0.0 0.0 (Math|Random|RandomFloatinRange 0.0 3.6e+02)) false false)
    (ChildActorComponent|SetChildActorClass _returnvalue_2 (Variables|Default|GetlocalbpClass))))