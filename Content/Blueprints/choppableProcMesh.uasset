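; Actor for a choppable procedural mesh piece that can be picked up and dropped.
; The attach event takes a procedural mesh, turns on gravity, collision and damped physics simulation, then clears its first mesh section.
; Pickup attaches the actor's root to a supplied component and Drop detaches it, both keeping world transforms.
; Construction and Init are empty, and some attachment and convex collision nodes are left unconnected.
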(event Custom|attach
  (params (procmesh :type Procedural%20Mesh%20Component%20Object%20Reference))
  (Physics|SetEnableGravity procmesh true)
  (Collision|SetCollisionEnabled procmesh "QueryAndPhysics")
  (Physics|SetSimulatePhysics procmesh true)
  (Class|PrimitiveComponent|SetLinearDamping procmesh 1.0)
  (Class|PrimitiveComponent|SetAngularDamping procmesh 1.0)
  (Class|ProceduralMeshComponent|ClearMeshSection procmesh))

(event EventBeginPlay)

(event EventPickup
  (params (AttachTo :type Scene%20Component%20Object%20Reference))
  (Transformation|AttachComponentToComponent (VehicleSound|GetRootComponent) AttachTo "None" "KeepWorld" "KeepWorld" "KeepWorld" false))

(event EventDrop
  (Transformation|DetachFromActor "KeepWorld" "KeepWorld" "KeepWorld"))

(fn ConstructionScript)

(fn Init)