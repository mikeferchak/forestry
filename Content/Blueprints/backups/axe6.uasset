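; A VR axe that motion controllers pick up and drop, toggling physics, and that chops procedural-mesh choppable actors on impact.
; Hits above an impulse threshold, gated by a short cooldown flag, call ChopEvent on the target and play a random impulse-scaled chop sound.
; Slice, DuplicateActor and RandomHitSound are defined but not called here; Slice cuts a procedural mesh along the axe's orientation into physics pieces.
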(event OnComponentHit(StaticMeshComponent)
  (params (HitComponent :type Primitive%20Component%20Object%20Reference) (OtherActor :type Actor%20Object%20Reference) (OtherComp :type Primitive%20Component%20Object%20Reference) (NormalImpulse :type Vector) (Hit :type Hit%20Result%20Structure%20%28by%20ref%29))
  (bind _shouldchop (CallFunction|ShouldChop NormalImpulse))
  (if _shouldchop
    (bind _aschoppable (Utilities|Casting|CastTochoppable OtherActor))
    (bind _asprocedural_mesh_component (Utilities|Casting|CastToProceduralMeshComponent OtherComp))
    (Default|ChopEvent _aschoppable Hit (Variables|Debug|GetStaticMeshComponent) _asprocedural_mesh_component)
    (CallFunction|RandomChopSound NormalImpulse Hit)
    (Utilities|FlowControl|Delay 0.2)
    (Variables|Default|Setcanchop true)))

(event EventBeginPlay
  (Physics|SetSimulatePhysics (Variables|Debug|GetStaticMeshComponent) (Variables|Default|Getinit_with_physics)))

(event EventPickup
  (params (AttachTo :type Scene%20Component%20Object%20Reference))
  (Physics|SetSimulatePhysics (Variables|Debug|GetStaticMeshComponent) false)
  (Transformation|AttachComponentToComponent (VehicleSound|GetRootComponent) AttachTo "None" "KeepWorld" "KeepWorld" "KeepWorld" false))

(event EventDrop
  (Physics|SetSimulatePhysics (Variables|Debug|GetStaticMeshComponent) true)
  (Transformation|DetachFromActor "KeepWorld" "KeepWorld" "KeepWorld"))

(fn ConstructionScript)

(fn Slice
  (params (sliced_object :type Primitive%20Component%20Object%20Reference) (hit :type Hit%20Result%20Structure) (sliced_actor :type Actor%20Object%20Reference) (invert_vector :type Boolean))
  (bind _returnvalue (Actor|GetComponentbyClass sliced_actor "/Script/ProceduralMeshComponent.ProceduralMeshComponent"))
  (LocalVariables|SetplaneNormalMultiplier "-1.000000,-1.000000,-1.000000")
  (bind _outotherhalfprocmesh (Class|KismetProceduralMeshLibrary|SliceProceduralMesh _returnvalue (.ImpactPoint (Collision|BreakHitResult hit)) (* (Math|Vector|GetRightVector (Transformation|GetWorldRotation (Variables|Debug|GetStaticMeshComponent))) (LocalVariables|GetplaneNormalMultiplier)) true "CreateNewSectionForCap"))
  (bind _output_get (LocalVariables|SetoutProcMesh _outotherhalfprocmesh))
  (Utilities|FlowControl|Sequence
    (:then_0
      (Physics|SetEnableGravity _output_get true))
    (:then_1
      (Collision|SetCollisionEnabled _output_get "QueryAndPhysics"))
    (:then_2
      (Physics|SetSimulatePhysics _output_get true))
    (:then_3
      (Class|PrimitiveComponent|SetLinearDamping _output_get 5.0))
    (:then_4
      (Class|PrimitiveComponent|SetAngularDamping _output_get 5.0))
    (:then_5
      (bind _returnvalue_2 (Game|SpawnActorfromClass "/Game/Blueprints/choppableProcMesh.choppableProcMesh_C" (Transformation|GetWorldTransform _output_get) "Undefined" 0 0))
      (Default|Attach _returnvalue_2 (LocalVariables|GetoutProcMesh)))
    (:then_7
      (Development|PrintString (Utilities|String|ToString(Integer) (Class|ProceduralMeshComponent|GetNumSections _returnvalue))))
    (:then_8
      (Development|PrintString (Utilities|String|ToString(Integer) (Class|SceneComponent|GetNumChildrenComponents _returnvalue))))
    (:then_9
      (return))))

(fn RandomChopSound
  (params (impulse :type Vector) (hit :type Hit%20Result%20Structure))
  (bind _chopsounds (Variables|Default|GetchopSounds))
  (Audio|PlaySoundatLocation (Utilities|Array|Get(acopy) _chopsounds (Math|Random|RandomIntegerinRange 0 (- (Utilities|Array|Length _chopsounds) 1))) (.ImpactPoint (Collision|BreakHitResult hit)) "0, 0, 0" (Math|Float|Clamp(Float) (/ (Math|Vector|VectorLength impulse) 2.5e+03) 0.0 5.0) 1.0 0.0 "/Game/audio/chopEffectAttenuation.chopEffectAttenuation")
  (return))

(fn RandomHitSound
  (params (impulse :type Vector) (hit :type Hit%20Result%20Structure))
  (bind _hitsounds (Variables|Default|GethitSounds))
  (Audio|PlaySoundatLocation (Utilities|Array|Get(acopy) _hitsounds (Math|Random|RandomIntegerinRange 0 (- (Utilities|Array|Length _hitsounds) 1))) (.ImpactPoint (Collision|BreakHitResult hit)) "0, 0, 0" (Math|Float|Clamp(Float) (/ (Math|Vector|VectorLength impulse) 2.5e+03) 0.0 5.0) 1.0 0.0 "/Game/audio/chopEffectAttenuation.chopEffectAttenuation")
  (return))

(fn ShouldChop
  (params (impulse :type Vector))
  (if (> (Math|Vector|VectorLength impulse) (Variables|Default|GetchopThreshold))
    (if (Variables|Default|Getcanchop)
      (Variables|Default|Setcanchop false)
      (return true)
      (else
        _)))
  (return false))

(fn DuplicateActor
  (params (actor :type Actor%20Object%20Reference))
  (bind _output_get (LocalVariables|SetactorRef actor))
  (bind _asprocedural_mesh_component (Utilities|Casting|CastToProceduralMeshComponent (VehicleSound|GetRootComponent _output_get))
    (:then
      (Utilities|FlowControl|Sequence
        (:then_0
          (bind _returnvalue (Game|SpawnActorfromClass "/Game/Blueprints/choppableProcMesh.choppableProcMesh_C" (Transformation|GetWorldTransform _asprocedural_mesh_component) "AlwaysSpawn" 0 0)))
        (:then_1
          (bind _returnvalue_2 (Game|SpawnActorfromClass "/Game/Blueprints/choppableProcMesh.choppableProcMesh_C" (Transformation|GetWorldTransform _asprocedural_mesh_component) "AlwaysSpawn" 0 0)))
        (:then_2
          (Actor|DestroyActor (LocalVariables|GetactorRef))
          (return _returnvalue _returnvalue_2))))
    (:CastFailed
      (return 0 0))))