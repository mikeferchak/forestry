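; A VR-style pickup axe that chops procedural meshes on hard impacts, with physics toggled as a motion controller grabs or drops it.
; Hits above an impulse threshold, gated by a short cooldown, slice the struck ProceduralMeshComponent at the impact point along the axe's right-vector plane.
; The new half gets a log cap material and damped physics, and a random chop sound scales with impulse.
; RandomHitSound and some slice-spawning nodes are unused.
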(event OnComponentHit(StaticMeshComponent)
  (params (HitComponent :type Primitive%20Component%20Object%20Reference) (OtherActor :type Actor%20Object%20Reference) (OtherComp :type Primitive%20Component%20Object%20Reference) (NormalImpulse :type Vector) (Hit :type Hit%20Result%20Structure%20%28by%20ref%29))
  (if (> (Math|Vector|VectorLength NormalImpulse) (Variables|Default|GetchopThreshold))
    (if (Variables|Default|Getcanchop)
      (Variables|Default|Setcanchop false)
      (CallFunction|Slice OtherComp NormalImpulse Hit)
      (CallFunction|RandomChopSound NormalImpulse Hit)
      (Utilities|FlowControl|Delay 0.2)
      (Variables|Default|Setcanchop true))))

(event EventBeginPlay
  (Physics|SetSimulatePhysics (Variables|Debug|GetStaticMeshComponent) (Variables|Default|Getinit_with_physics)))

(event EventPickup
  (params (AttachTo :type Scene%20Component%20Object%20Reference))
  (Physics|SetSimulatePhysics (Variables|Debug|GetStaticMeshComponent) false)
  (Transformation|AttachComponentToComponent (VehicleSound|GetRootComponent) AttachTo "None" "KeepWorld" "KeepWorld" "KeepWorld" false))

(event EventDrop
  (Physics|SetSimulatePhysics (Variables|Debug|GetStaticMeshComponent) true)
  (Transformation|DetachFromActor "KeepWorld" "KeepWorld" "KeepWorld"))

(fn ConstructionScript)

(fn Slice
  (params (sliced_object :type Primitive%20Component%20Object%20Reference) (impulse :type Vector) (hit :type Hit%20Result%20Structure))
  (bind _asprocedural_mesh_component (Utilities|Casting|CastToProceduralMeshComponent sliced_object))
  (bind _outotherhalfprocmesh (Class|KismetProceduralMeshLibrary|SliceProceduralMesh _asprocedural_mesh_component (.ImpactPoint (Collision|BreakHitResult hit)) (Math|Vector|GetRightVector (Transformation|GetWorldRotation (Variables|Debug|GetStaticMeshComponent))) true "CreateNewSectionForCap" "/Game/materials/log_mat_Inst.log_mat_Inst"))
  (LocalVariables|SetoutProcMesh _outotherhalfprocmesh)
  (Physics|SetEnableGravity (LocalVariables|GetoutProcMesh) true)
  (Collision|SetCollisionEnabled (LocalVariables|GetoutProcMesh) "QueryAndPhysics")
  (Physics|SetSimulatePhysics (LocalVariables|GetoutProcMesh) true)
  (Class|PrimitiveComponent|SetLinearDamping (LocalVariables|GetoutProcMesh) 5.0)
  (Class|PrimitiveComponent|SetAngularDamping (LocalVariables|GetoutProcMesh) 5.0)
  (return (LocalVariables|GetoutProcMesh)))

(fn RandomChopSound
  (params (impulse :type Vector) (hit :type Hit%20Result%20Structure))
  (bind _chopsounds (Variables|Default|GetchopSounds))
  (Audio|PlaySoundatLocation (Utilities|Array|Get(acopy) _chopsounds (Math|Random|RandomIntegerinRange 0 (- (Utilities|Array|Length _chopsounds) 1))) (.ImpactPoint (Collision|BreakHitResult hit)) "0, 0, 0" (Math|Float|Clamp(Float) (/ (Math|Vector|VectorLength impulse) 2.5e+03) 0.0 5.0) 1.0 0.0 "/Game/audio/chopEffectAttenuation.chopEffectAttenuation")
  (return))

(fn RandomHitSound
  (params (impulse :type Vector) (hit :type Hit%20Result%20Structure))
  (bind _hitsounds (Variables|Default|GethitSounds))
  (Audio|PlaySoundatLocation (Utilities|Array|Get(acopy) _hitsounds (Math|Random|RandomIntegerinRange 0 (- (Utilities|Array|Length _hitsounds) 1))) (.ImpactPoint (Collision|BreakHitResult hit)) "0, 0, 0" (Math|Float|Clamp(Float) (/ (Math|Vector|VectorLength impulse) 2.5e+03) 0.0 5.0) 1.0 0.0 "/Game/audio/chopEffectAttenuation.chopEffectAttenuation")
  (return))