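; Grabbable axe that chops foliage and procedural meshes on impact, with collision disabled until first pickup.
; Component hits that pass an impulse threshold and Canchop flag swap the struck foliage instance for a spawned Choppable, or target an existing one.
; The Choppable's ChopEvent receives the hit and axe mesh, and a random chop sound plays, scaled by impulse.
; Older slice, duplicate and macro versions remain uncalled here.
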(event OnComponentHit(StaticMeshComponent)
  (params (HitComponent :type Primitive%20Component%20Object%20Reference) (OtherActor :type Actor%20Object%20Reference) (OtherComp :type Primitive%20Component%20Object%20Reference) (NormalImpulse :type Vector) (Hit :type Hit%20Result%20Structure%20%28by%20ref%29))
  (Utilities|FlowControl|Sequence
    (:then_0
      (Variables|Default|Setcanchop true))
    (:then_1
      (CallFunction|TrytoChopFoliage Hit OtherActor OtherComp NormalImpulse))
    (:then_2
      (CallFunction|TrytoChopProcMesh OtherActor OtherComp NormalImpulse Hit))
    (:then_3
      (Variables|Default|Setcanchop false)
      (Utilities|FlowControl|Delay 0.2)
      (Variables|Default|Setcanchop true))))

(event EventBeginPlay
  (bind _staticmeshcomponent (Variables|Debug|GetStaticMeshComponent))
  (Physics|SetSimulatePhysics _staticmeshcomponent (Variables|Default|Getinit_with_physics))
  (Collision|SetCollisionEnabled _staticmeshcomponent "NoCollision"))

(event EventPickupComponent
  (params (AttachTo :type Scene%20Component%20Object%20Reference) (Component :type Primitive%20Component%20Object%20Reference))
  (Physics|SetSimulatePhysics Component false)
  (Collision|SetCollisionEnabled (Variables|Debug|GetStaticMeshComponent) "QueryAndPhysics")
  (Transformation|AttachComponentToComponent Component AttachTo "None" "KeepWorld" "KeepWorld" "KeepWorld" false)
  (Variables|Default|SethasBeenGripped true))

(event EventDropComponent
  (params (component :type Primitive%20Component%20Object%20Reference))
  (Physics|SetSimulatePhysics component true)
  (Transformation|DetachFromComponent component "KeepRelative" "KeepRelative" "KeepRelative" true))

(fn ConstructionScript)

(fn SliceUNUSED
  (params (sliced_object :type Primitive%20Component%20Object%20Reference) (hit :type Hit%20Result%20Structure) (sliced_actor :type Actor%20Object%20Reference) (invert_vector :type Boolean))
  (LocalVariables|SetplaneNormalMultiplier "-1.000000,-1.000000,-1.000000")
  (bind _outotherhalfprocmesh (Class|KismetProceduralMeshLibrary|SliceProceduralMesh (Actor|GetComponentbyClass sliced_actor "/Script/ProceduralMeshComponent.ProceduralMeshComponent") (.ImpactPoint (Collision|BreakHitResult hit)) (* (Math|Vector|GetRightVector (Transformation|GetWorldRotation (Variables|Debug|GetStaticMeshComponent))) (LocalVariables|GetplaneNormalMultiplier)) true "CreateNewSectionForCap"))
  (LocalVariables|SetoutProcMesh _outotherhalfprocmesh)
  (Utilities|FlowControl|Sequence
    (:then_0
      (Physics|SetEnableGravity (LocalVariables|GetoutProcMesh) true))
    (:then_1
      (Collision|SetCollisionEnabled (LocalVariables|GetoutProcMesh) "QueryAndPhysics"))
    (:then_2
      (Physics|SetSimulatePhysics (LocalVariables|GetoutProcMesh) true))
    (:then_3
      (Class|PrimitiveComponent|SetLinearDamping (LocalVariables|GetoutProcMesh) 5.0))
    (:then_4
      (Class|PrimitiveComponent|SetAngularDamping (LocalVariables|GetoutProcMesh) 5.0))
    (:then_5
      (bind _returnvalue (Game|SpawnActorfromClass "/Game/Blueprints/choppableProcMesh.choppableProcMesh_C" (Transformation|GetWorldTransform (LocalVariables|GetoutProcMesh)) "Undefined" 0 0))
      (Default|Attach _returnvalue (LocalVariables|GetoutProcMesh))
      (return))))

(fn RandomChopSound
  (params (impulse :type Vector) (hit :type Hit%20Result%20Structure))
  (bind _chopsounds (Variables|Default|GetchopSounds))
  (Audio|PlaySoundatLocation (Utilities|Array|Get(acopy) _chopsounds (Math|Random|RandomIntegerinRange 0 (- (Utilities|Array|Length _chopsounds) 1))) (.ImpactPoint (Collision|BreakHitResult hit)) "0, 0, 0" (Math|Float|Clamp(Float) (/ (Math|Vector|VectorLength impulse) 2.5e+03) 0.0 5.0) 1.0 0.0 "/Game/audio/chopEffectAttenuation.chopEffectAttenuation")
  (return))

(fn RandomHitSound
  (params (impulse :type Vector) (hit :type Hit%20Result%20Structure))
  (bind _hitsounds (Variables|Default|GethitSounds))
  (Audio|PlaySoundatLocation (Utilities|Array|Get(acopy) _hitsounds (Math|Random|RandomIntegerinRange 0 (- (Utilities|Array|Length _hitsounds) 1))) (.ImpactPoint (Collision|BreakHitResult hit)) "0, 0, 0" (Math|Float|Clamp(Float) (/ (Math|Vector|VectorLength impulse) 2.5e+03) 0.0 5.0) 1.0 0.0 "/Game/audio/chopEffectAttenuation.chopEffectAttenuation")
  (return))

(fn ShouldChop
  (params (impulse :type Vector))
  (if (> (Math|Vector|VectorLength impulse) (Variables|Default|GetchopThreshold))
    (if (Variables|Default|Getcanchop)
      (Variables|Default|Setcanchop false)
      (return true)
      (else
        _)))
  (return false))

(fn DuplicateActor
  (params (actor :type Actor%20Object%20Reference))
  (bind _output_get (LocalVariables|SetactorRef actor))
  (bind _asprocedural_mesh_component (Utilities|Casting|CastToProceduralMeshComponent (VehicleSound|GetRootComponent _output_get))
    (:then
      (Utilities|FlowControl|Sequence
        (:then_0
          (bind _returnvalue (Game|SpawnActorfromClass "/Game/Blueprints/choppableProcMesh.choppableProcMesh_C" (Transformation|GetWorldTransform _asprocedural_mesh_component) "AlwaysSpawn" 0 0)))
        (:then_1
          (bind _returnvalue_2 (Game|SpawnActorfromClass "/Game/Blueprints/choppableProcMesh.choppableProcMesh_C" (Transformation|GetWorldTransform _asprocedural_mesh_component) "AlwaysSpawn" 0 0)))
        (:then_2
          (Actor|DestroyActor (LocalVariables|GetactorRef))
          (return _returnvalue _returnvalue_2))))
    (:CastFailed
      (return 0 0))))

(fn TrytoChopFoliage
  (params (hit :type Hit%20Result%20Structure) (actor :type Actor%20Object%20Reference) (component :type Primitive%20Component%20Object%20Reference) (impulse :type Vector))
  (LocalVariables|Set_hit hit)
  (LocalVariables|Set_actor actor)
  (LocalVariables|Set_component component)
  (LocalVariables|Set_impulse impulse)
  (bind _asinstanced_static_mesh_component (Utilities|Casting|CastToInstancedStaticMeshComponent (LocalVariables|Get_component)))
  (LocalVariables|SetfoliageInstancedComponent _asinstanced_static_mesh_component)
  (LocalVariables|SethitItemIndex (.HitItem (Collision|BreakHitResult (LocalVariables|Get_hit))))
  (bind _shouldchop (CallFunction|ShouldChop (LocalVariables|Get_impulse)))
  (if _shouldchop
    (bind _returnvalue (Game|SpawnActorfromClass "/Game/Blueprints/choppable.choppable_C" (.OutInstanceTransform (Components|InstancedStaticMesh|GetInstanceTransform (LocalVariables|GetfoliageInstancedComponent) (LocalVariables|GethitItemIndex) true)) "Undefined" 0 0))
    (LocalVariables|SetnewChoppableActor _returnvalue)
    (Variables|/Game/Blueprints/choppable.choppable_C|Setmesh (LocalVariables|GetnewChoppableActor) (Variables|/Script/Engine.StaticMeshComponent|GetStaticMesh (LocalVariables|GetfoliageInstancedComponent)))
    (Default|ReinitChoppableObjectEvent (LocalVariables|GetnewChoppableActor))
    (Default|ChopEvent (LocalVariables|GetnewChoppableActor) (LocalVariables|Get_hit) (Variables|Debug|GetStaticMeshComponent) (Variables|/Game/Blueprints/choppable.choppable_C|GetProceduralMesh (LocalVariables|GetnewChoppableActor)))
    (Class|InstancedStaticMeshComponent|RemoveInstance (LocalVariables|GetfoliageInstancedComponent) (LocalVariables|GethitItemIndex))
    (CallFunction|RandomChopSound (LocalVariables|Get_impulse) (LocalVariables|Get_hit))))

(fn TrytoChopProcMesh
  (params (actor :type Actor%20Object%20Reference) (component :type Primitive%20Component%20Object%20Reference) (inpulse :type Vector) (hit :type Hit%20Result%20Structure))
  (bind _asprocedural_mesh_component (Utilities|Casting|CastToProceduralMeshComponent component))
  (bind _shouldchop (CallFunction|ShouldChop inpulse))
  (if _shouldchop
    (bind _aschoppable (Utilities|Casting|CastTochoppable actor))
    (Default|ChopEvent _aschoppable hit (Variables|Debug|GetStaticMeshComponent) _asprocedural_mesh_component)
    (CallFunction|RandomChopSound inpulse hit)))