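; Choppable prop that can be picked up, dropped and sliced apart with an axe.
; Construction copies a configurable static mesh into a procedural mesh with optional physics, gravity and collision.
; Pickup and drop events toggle physics and attachment for the actor or single components.
; Chop slices the hit component at the impact point along a plane from the target's right vector, capping the new half and making it a damped physics piece.
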(event Custom|reinitChoppableObjectEvent
  (CallFunction|Initialize))

(event Custom|chopEvent
  (params (hit :type Hit%20Result%20Structure) (axe :type Static%20Mesh%20Component%20Object%20Reference) (component :type Procedural%20Mesh%20Component%20Object%20Reference))
  (Utilities|Chop axe hit component))

(event EventBeginPlay)

(event EventPickup
  (params (AttachTo :type Scene%20Component%20Object%20Reference))
  (Physics|SetSimulatePhysics (Variables|Default|GetProceduralMesh) false)
  (Transformation|AttachComponentToComponent (VehicleSound|GetRootComponent) AttachTo "None" "KeepWorld" "KeepWorld" "KeepWorld" false))

(event EventDrop
  (Physics|SetSimulatePhysics (Variables|Default|GetProceduralMesh) true)
  (Transformation|DetachFromActor "KeepWorld" "KeepWorld" "KeepWorld"))

(event EventPickupComponent
  (params (AttachTo :type Scene%20Component%20Object%20Reference) (Component :type Primitive%20Component%20Object%20Reference))
  (Physics|SetSimulatePhysics Component false)
  (Transformation|AttachComponentToComponent Component AttachTo "None" "KeepWorld" "KeepWorld" "KeepWorld" false))

(event EventDropComponent
  (params (component :type Primitive%20Component%20Object%20Reference))
  (Physics|SetSimulatePhysics (Variables|Default|GetProceduralMesh) true)
  (Transformation|DetachFromComponent component "KeepWorld" "KeepWorld" "KeepWorld" true)
  (Transformation|DetachFromActor "KeepRelative" "KeepRelative" "KeepRelative"))

(fn ConstructionScript
  (CallFunction|Initialize))

(fn Initialize
  (Components|StaticMesh|SetStaticMesh (Variables|Default|Getstaticmeshref) (Variables|Default|Getmesh))
  (Class|PrimitiveComponent|SetMassOverrideinKg (Variables|Default|Getstaticmeshref) "None" 1e+02 true)
  (Class|KismetProceduralMeshLibrary|CopyProceduralMeshfromStaticMeshComponent (Variables|Default|Getstaticmeshref) 0 (Variables|Default|GetProceduralMesh) (Variables|Default|GetcreateCollision))
  (Physics|SetEnableGravity (Variables|Default|GetProceduralMesh) (Variables|Default|Getgravity))
  (Physics|SetSimulatePhysics (Variables|Default|GetProceduralMesh) (Variables|Default|Getphysics)))