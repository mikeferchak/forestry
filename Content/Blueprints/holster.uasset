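; VR holster actor that supplies axes from four body-style slots: left, right, back-left and back-right.
; When a BP_MotionController enters a slot, Spawnandattach rumbles it, spawns an Axe attached to that placeholder and sets its mesh to query-only collision.
; On end overlap, the slot's stored axe is destroyed unless it has been gripped, so axes exist on demand.
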(event OnComponentBeginOverlap(leftPlaceholder)
  (params (OverlappedComponent :type Primitive%20Component%20Object%20Reference) (OtherActor :type Actor%20Object%20Reference) (OtherComp :type Primitive%20Component%20Object%20Reference) (OtherBodyIndex :type Integer) (bFromSweep :type Boolean) (SweepResult :type Hit%20Result%20Structure%20%28by%20ref%29))
  (bind _returnvalue (CallFunction|Spawnandattach (Variables|Default|GetleftPlaceholder) OtherActor)))

(event OnComponentEndOverlap(leftPlaceholder)
  (params (OverlappedComponent :type Primitive%20Component%20Object%20Reference) (OtherActor :type Actor%20Object%20Reference) (OtherComp :type Primitive%20Component%20Object%20Reference) (OtherBodyIndex :type Integer))
  (Utilities|IsValid (stale OnComponentBeginOverlap(leftPlaceholder) _returnvalue)
    (:Is%20Valid
      (if (not (Variables|/Game/Blueprints/axe.axe_C|GethasBeenGripped (stale OnComponentBeginOverlap(leftPlaceholder) _returnvalue)))
        (Actor|DestroyActor (stale OnComponentBeginOverlap(leftPlaceholder) _returnvalue))))))

(event OnComponentBeginOverlap(rightPlaceholder)
  (params (OverlappedComponent :type Primitive%20Component%20Object%20Reference) (OtherActor :type Actor%20Object%20Reference) (OtherComp :type Primitive%20Component%20Object%20Reference) (OtherBodyIndex :type Integer) (bFromSweep :type Boolean) (SweepResult :type Hit%20Result%20Structure%20%28by%20ref%29))
  (bind _returnvalue (CallFunction|Spawnandattach (Variables|Default|GetrightPlaceholder) OtherActor)))

(event OnComponentEndOverlap(rightPlaceholder)
  (params (OverlappedComponent :type Primitive%20Component%20Object%20Reference) (OtherActor :type Actor%20Object%20Reference) (OtherComp :type Primitive%20Component%20Object%20Reference) (OtherBodyIndex :type Integer))
  (Utilities|IsValid (stale OnComponentBeginOverlap(rightPlaceholder) _returnvalue)
    (:Is%20Valid
      (if (not (Variables|/Game/Blueprints/axe.axe_C|GethasBeenGripped (stale OnComponentBeginOverlap(rightPlaceholder) _returnvalue)))
        (Actor|DestroyActor (stale OnComponentBeginOverlap(rightPlaceholder) _returnvalue))))))

(event OnComponentEndOverlap(backPlaceholderRight)
  (params (OverlappedComponent :type Primitive%20Component%20Object%20Reference) (OtherActor :type Actor%20Object%20Reference) (OtherComp :type Primitive%20Component%20Object%20Reference) (OtherBodyIndex :type Integer))
  (Utilities|IsValid (stale OnComponentBeginOverlap(backPlaceholderRight) _returnvalue)
    (:Is%20Valid
      (if (not (Variables|/Game/Blueprints/axe.axe_C|GethasBeenGripped (stale OnComponentBeginOverlap(backPlaceholderRight) _returnvalue)))
        (Actor|DestroyActor (stale OnComponentBeginOverlap(backPlaceholderRight) _returnvalue))))))

(event OnComponentBeginOverlap(backPlaceholderLeft)
  (params (OverlappedComponent :type Primitive%20Component%20Object%20Reference) (OtherActor :type Actor%20Object%20Reference) (OtherComp :type Primitive%20Component%20Object%20Reference) (OtherBodyIndex :type Integer) (bFromSweep :type Boolean) (SweepResult :type Hit%20Result%20Structure%20%28by%20ref%29))
  (bind _returnvalue (CallFunction|Spawnandattach (Variables|Default|GetbackPlaceholderLeft) OtherActor)))

(event OnComponentEndOverlap(backPlaceholderLeft)
  (params (OverlappedComponent :type Primitive%20Component%20Object%20Reference) (OtherActor :type Actor%20Object%20Reference) (OtherComp :type Primitive%20Component%20Object%20Reference) (OtherBodyIndex :type Integer))
  (Utilities|IsValid (stale OnComponentBeginOverlap(backPlaceholderLeft) _returnvalue)
    (:Is%20Valid
      (if (not (Variables|/Game/Blueprints/axe.axe_C|GethasBeenGripped (stale OnComponentBeginOverlap(backPlaceholderLeft) _returnvalue)))
        (Actor|DestroyActor (stale OnComponentBeginOverlap(backPlaceholderLeft) _returnvalue))))))

(event OnComponentBeginOverlap(backPlaceholderRight)
  (params (OverlappedComponent :type Primitive%20Component%20Object%20Reference) (OtherActor :type Actor%20Object%20Reference) (OtherComp :type Primitive%20Component%20Object%20Reference) (OtherBodyIndex :type Integer) (bFromSweep :type Boolean) (SweepResult :type Hit%20Result%20Structure%20%28by%20ref%29))
  (bind _returnvalue (CallFunction|Spawnandattach (Variables|Default|GetbackPlaceholderRight) OtherActor)))

(fn ConstructionScript)

(fn Spawnandattach
  (params (Target :type Scene%20Component%20Object%20Reference) (overlappingActor :type Actor%20Object%20Reference))
  (Utilities|IsValid Target
    (:Is%20Valid
      (Utilities|IsValid overlappingActor
        (:Is%20Valid
          (bind _asbp_motion_controller (Utilities|Casting|CastToBP_MotionController overlappingActor)
            (:then
              (Default|RumbleController _asbp_motion_controller 1.0)
              (bind _returnvalue (Game|SpawnActorfromClass "/Game/Blueprints/axe.axe_C" (Transformation|GetWorldTransform Target) "Undefined" 0 0))
              (Transformation|AttachComponentToComponent _returnvalue Target "None" "KeepWorld" "KeepWorld" "KeepWorld" false)
              (Collision|SetCollisionEnabled (Variables|/Script/Engine.StaticMeshActor|GetStaticMeshComponent _returnvalue) "QueryOnly")
              (return _returnvalue))
            (:CastFailed
              (return 0))))))))