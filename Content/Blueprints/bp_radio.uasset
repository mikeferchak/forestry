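; A VR radio prop that plays a music track and can be picked up and dropped with a motion controller.
; On BeginPlay it spawns the track attached to its static mesh, assigns the ChopEffectAttenuation settings and plays it.
; Pickup, called by BP_MotionController, turns off physics and attaches the root component to the given component, keeping its world transform.
; Drop re-enables physics and detaches the actor.
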(event EventBeginPlay
  (bind _returnvalue (Audio|SpawnSoundAttached "/Game/audio/soundtrack/04_Hard_Time_Killin__Floor_Blues_mp3.04_Hard_Time_Killin__Floor_Blues_mp3" (Variables|Debug|GetStaticMeshComponent)))
  (Variables|/Script/Engine.AudioComponent|SetAttenuationSettings _returnvalue "/Game/audio/chopEffectAttenuation.chopEffectAttenuation")
  (Audio|Components|Audio|Play _returnvalue 0.0))

(event Collision|EventActorBeginOverlap
  (params (OtherActor :type Actor%20Object%20Reference)))

(event EventTick
  (params (DeltaSeconds :type Float%20%28single-precision%29)))

(event EventPickup
  (params (AttachTo :type Scene%20Component%20Object%20Reference))
  (Physics|SetSimulatePhysics (Variables|Debug|GetStaticMeshComponent) false)
  (Transformation|AttachComponentToComponent (VehicleSound|GetRootComponent) AttachTo "None" "KeepWorld" "KeepWorld" "KeepWorld" false))

(event EventDrop
  (Physics|SetSimulatePhysics (Variables|Debug|GetStaticMeshComponent) true)
  (Transformation|DetachFromActor "KeepWorld" "KeepWorld" "KeepWorld"))

(fn ConstructionScript)